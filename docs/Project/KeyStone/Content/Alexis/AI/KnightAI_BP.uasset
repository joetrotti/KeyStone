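; Knight enemy AI character that slashes the player with an attached sword and shows a health bar and reticle on lock-on.
; An overlap box gates DamagePlayer, while ATK_01 turns the knight toward its target and plays the slash montage.
; Damage updates the health bar; at zero health the knight ragdolls, is destroyed and clears player lock-on.
; Health is copied to the game instance every Tick and restored from the save on BeginPlay.
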(event `ATK_01`
  (params (Target :type "Actor Object Reference"))
  (bind (_returnvalue_roll _returnvalue_pitch _returnvalue_yaw) (`KismetMathLibrary.BreakRotator` (`KismetMathLibrary.FindLookAtRotation` (`self.K2_GetActorLocation`) (`self.K2_GetActorLocation` Target))))
  ;[1 1 1] ATTACK 1
  (`|ExecutionSequence`
    (:`then_0`
      (`/Engine/EditorBlueprintResources/StandardMacros.IsValid` Target
        (:`Is Valid`
          (`self.K2_SetActorRotation` (`KismetMathLibrary.MakeRotator` 0.0 0.0 _returnvalue_yaw)))))
    (:`then_1`
      (`self.PlayAnimMontage` "/Game/Alexis/AI/aiAnimations/slashKnight.slashKnight")
      (bind _asplayer (cast `/Game/Player` (`GameplayStatics.GetPlayerPawn` 0)))
      (if (not (`/Game/Player.IsDead1` _asplayer))
        (bind _asplayer_2 (cast `/Game/Player` (`GameplayStatics.GetPlayerPawn` 0)))
        (if (not (`/Game/Player.isDead1` _asplayer_2))
          (`GameplayStatics.PlaySoundAtLocation` "/Game/SoundForKeyStone/Grunts/voice_male_effort_grunt_01.voice_male_effort_grunt_01" (`self.K2_GetActorLocation`) (struct) 1.0 0.75 0.0 null null null))))))

(event `self.ReceiveTick`
  (params (DeltaSeconds :type "Float (single-precision)"))
  ;[1 1 1] Continuously Save Health
  (bind _asmy_game_instance (cast `/Game/Tanner/MainMenu/MyGameInstance` (`GameplayStatics.GetGameInstance`)))
  (set `/Game/Tanner/MainMenu/MyGameInstance.KnightHealthGameInst` (`self.Health`) _asmy_game_instance))

(event `self.ReceiveBeginPlay`
  (`|ExecutionSequence`
    (:`then_0`
      ;[1 1 1] Attaches Sword to Enemy AI
      (bind _returnvalue (`|SpawnActorFromClass` "/Game/Alexis/AI/EnemySword.EnemySword_C" (`SceneComponent.GetSocketTransform` (`self.Mesh`) "weaponhand" "RTS_World") "Undefined" "OverrideRootScale" null null))
      (`self.K2_AttachToComponent` _returnvalue (`self.Mesh`) "weaponhand" "SnapToTarget" "SnapToTarget" "SnapToTarget" true)
      ;[1 1 1] For changing the enemies health when a save is loaded
      (`|ExecutionSequence`
        (:`then_0`
          (bind _asmy_game_instance (cast `/Game/Tanner/MainMenu/MyGameInstance` (`GameplayStatics.GetGameInstance`)))
          (bind _savegame (`AsyncActionHandleSaveGame.AsyncLoadGameFromSlot` (`/Game/Tanner/MainMenu/MyGameInstance.PointerToSave` _asmy_game_instance) (`/Game/Tanner/MainMenu/MyGameInstance.PointerToSaveInd` _asmy_game_instance))
            (:`Completed`
              (bind _asmy_save_game (cast `/Game/Tanner/SaveGame/MySaveGame` _savegame))
              (bind _output_get (set `self.Health` (`/Game/Tanner/SaveGame/MySaveGame.EnemyHealthKnight` _asmy_save_game)))
              (`KismetSystemLibrary.PrintString` (`KismetStringLibrary.Concat_StrStr` "EnemyHealth: " (`KismetStringLibrary.Conv_DoubleToString` _output_get)))
              (if (<= _output_get 0.0)
                (`KismetSystemLibrary.PrintString` "EnemyDeadOnSave")
                (`self.K2_DestroyActor`)))))))
    (:`then_1`
      ;[1 1 1] Creates reference to health bar
      (bind _asknight_health (cast `/Game/Alexis/AI/KnightHealth` (`WidgetComponent.GetUserWidgetObject` (`self.Healthbar`))))
      (bind _output_get_2 (set `self.As Knight Health` _asknight_health)))))

(event `self.Box.OnComponentBeginOverlap`
  (params (OverlappedComponent :type "PrimitiveComponent Object Reference") (OtherActor :type "Actor Object Reference") (OtherComp :type "PrimitiveComponent Object Reference") (OtherBodyIndex :type Integer) (bFromSweep :type Boolean) (SweepResult :type "HitResult Structure (by ref)"))
  ;[1 0.1453 0.1354] If overlap with box do damage if not dont do damage
  (bind _asplayer (cast `/Game/Player` OtherActor))
  (if (not (`/Game/Player.isDead1` _asplayer))
    (set `self.Player` _asplayer)
    (if (`self.ActorHasTag` _asplayer "Player")
      (`/Engine/EditorBlueprintResources/StandardMacros.DoOnce` false :!label _label
        (:`Completed`
          (set `self.IsAttackable` true))))))

(event `DamagePlayer`
  ;[1 0.1855 0.1557] Does Damage
  (if (`self.IsAttackable`)
    (`GameplayStatics.ApplyDamage` (`self.Player`) 10.0 null self)))

(event `Reset`
  ;[1 0.1453 0.1354] If overlap with box do damage if not dont do damage
  (goto _label :!via `Reset`))

(event `self.Box.OnComponentEndOverlap`
  (params (OverlappedComponent :type "PrimitiveComponent Object Reference") (OtherActor :type "Actor Object Reference") (OtherComp :type "PrimitiveComponent Object Reference") (OtherBodyIndex :type Integer))
  ;[1 0.1453 0.1354] If overlap with box do damage if not dont do damage
  (bind _asplayer (cast `/Game/Player` OtherActor))
  (if (not (`/Game/Player.isDead1` _asplayer))
    (set `self.Player` _asplayer)
    (`self.Reset`)
    (set `self.IsAttackable` false)))

(event `self.ReceiveAnyDamage`
  (params (Damage :type "Float (single-precision)") (DamageType :type "DamageType Object Reference") (InstigatedBy :type "Controller Object Reference") (DamageCauser :type "Actor Object Reference"))
  ;[0.7846 0.5094 1] Getting Hit/ Health Increments + Animation/Reaction to Gettting Hit
  (`AISense_Damage.ReportDamageEvent` self (`GameplayStatics.GetPlayerCharacter` 0))
  (bind _output_get (set `self.Health` (- (`self.Health`) Damage)))
  (set `/Game/Alexis/AI/KnightHealth.Health` _output_get (`self.As Knight Health`))
  (`AddComponent|NODE_AddParticleSystemComponent-0`)
  (if (<= (`self.Health`) 0.0)
    (`self.Kill Enemy`)
    (`/Engine/EditorBlueprintResources/StandardMacros.DoOnce` false
      (:`Completed`
        (`GameplayStatics.PlaySoundAtLocation` "/Game/SoundForKeyStone/Enemies/Zombie_In_Pain-SoundBible_com-134322253.Zombie_In_Pain-SoundBible_com-134322253" (`self.K2_GetActorLocation`) (struct) 1.0 0.5 0.0 null null null)
        (bind _asplayer (cast `/Game/Player` (`GameplayStatics.GetPlayerPawn` 0)))
        (set `/Game/Player.TargetLocked` false _asplayer)))))

(event `Kill Enemy`
  ;[1 1 1] Ragdolls the enemy
  (`self.Ragdoll_Death`)
  (`KismetSystemLibrary.Delay` 1.0)
  (`self.K2_DestroyActor`))

(event `/Game/Evan/KeystoneImport/LockOn/LockOnBPI.LockOnReticle`
  (params (`Locked On?` :type Boolean))
  (bind _lockon (`self.LockOn`))
  (bind _healthbar (`self.Healthbar`))
  (if `Locked On?`
    (`SceneComponent.SetHiddenInGame` _lockon false false)
    (`SceneComponent.SetHiddenInGame` _healthbar false false)
    (else
      (`SceneComponent.SetHiddenInGame` _lockon true false)
      (`SceneComponent.SetHiddenInGame` _healthbar true false))))

(fn `Ragdoll_Death`
  (`PrimitiveComponent.SetSimulatePhysics` (`self.Mesh`) true)
  (`CharacterMovementComponent.DisableMovement` (`self.CharacterMovement`)))

(fn `UserConstructionScript`)