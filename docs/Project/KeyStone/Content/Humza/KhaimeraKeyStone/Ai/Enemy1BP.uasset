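; Khaimera enemy Blueprint that attacks the player, takes damage and ragdolls before being destroyed on death.
; Attacks face the target with random montages and sounds, and damage uses a sphere overlap on Player-tagged pawns.
; Attacking shows a health bar and swaps dungeon music for Khaimera music, reverting after a retriggerable timeout or death.
; Health loads from the save game, killing it if depleted, and copies to the game instance every tick.
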(event `self.ReceiveBeginPlay`
  ;[1 1 1] Enemy Speed
  (`|ExecutionSequence`
    (:`then_0`
      (set `CharacterMovementComponent.MaxWalkSpeed` 450.0 (`self.CharacterMovement`))
      ;[1 1 1] For changing the enemies health when a save is loaded
      (`|ExecutionSequence`
        (:`then_0`
          (bind _asmy_game_instance (cast `/Game/Tanner/MainMenu/MyGameInstance` (`GameplayStatics.GetGameInstance`)))
          (bind _savegame (`AsyncActionHandleSaveGame.AsyncLoadGameFromSlot` (`/Game/Tanner/MainMenu/MyGameInstance.PointerToSave` _asmy_game_instance) (`/Game/Tanner/MainMenu/MyGameInstance.PointerToSaveInd` _asmy_game_instance))
            (:`Completed`
              (bind _asmy_save_game (cast `/Game/Tanner/SaveGame/MySaveGame` _savegame))
              (bind _output_get (set `self.Health` (`/Game/Tanner/SaveGame/MySaveGame.EnemyHealth` _asmy_save_game)))
              (if (<= _output_get 0.0)
                (`self.Kill Enemy`)))))))))

(event `self.ReceiveTick`
  (params (DeltaSeconds :type "Float (single-precision)"))
  ;[1 1 1] Always update the enemies health in a game instance
  (bind _asmy_game_instance (cast `/Game/Tanner/MainMenu/MyGameInstance` (`GameplayStatics.GetGameInstance`)))
  (set `/Game/Tanner/MainMenu/MyGameInstance.EnemyHealthGameInst` (`self.Health`) _asmy_game_instance))

(event `ATK_01`
  (params (Target :type "Actor Object Reference"))
  (bind (_returnvalue_roll _returnvalue_pitch _returnvalue_yaw) (`KismetMathLibrary.BreakRotator` (`KismetMathLibrary.FindLookAtRotation` (`self.K2_GetActorLocation`) (`self.K2_GetActorLocation` Target))))
  ;[1 1 1] ATTACK 1
  (`|ExecutionSequence`
    (:`then_0`
      (`/Engine/EditorBlueprintResources/StandardMacros.IsValid` Target
        (:`Is Valid`
          (`self.K2_SetActorRotation` (`KismetMathLibrary.MakeRotator` 0.0 0.0 _returnvalue_yaw)))))
    (:`then_1`
      (`self.PlayAnimMontage` (`|GetArrayItem` (`self.AttackArray`) (`KismetMathLibrary.RandomIntegerInRange` 0 3)))
      (`GameplayStatics.PlaySoundAtLocation` (`|GetArrayItem` (`self.SoundArray`) (`KismetMathLibrary.RandomIntegerInRange` 0 1)) (`self.K2_GetActorLocation`) (struct) 1.0 1.0 0.0 null null null))))

(event `HealthBarRestartTimer`
  ;[1 1 1] HealthBar
  (`KismetSystemLibrary.RetriggerableDelay` 15.0)
  (`Widget.RemoveFromParent` (`self.KhimeraHealthBar`))
  (set `self.healthBarCreated?` false)
  (`AudioComponent.FadeOut` (`self.KhaimeraAudioComponent`) 3.0 0.0 "Linear")
  (bind _asplayer (cast `/Game/Player` (`GameplayStatics.GetPlayerCharacter` 0)))
  (`GameplayStatics.PlaySound2D` (`/Game/Player.DungeonCue` _asplayer) 1.0 1.0 0.0 null null))

(event `DoDamage`
  ;[1 0.2511 0.1614] Do Damage
  (if (not (`self.healthBarCreated?`))
    (bind _returnvalue (`|CreateWidget` "/Game/KeystoneThirdPerson/Blueprints/HUD/KhaimeraHealthbar.KhaimeraHealthbar_C"))
    (`UserWidget.AddToViewport` _returnvalue 0)
    (set `/Game/KeystoneThirdPerson/Blueprints/HUD/KhaimeraHealthbar.Target Actor` self _returnvalue)
    (set `self.KhimeraHealthBar` _returnvalue)
    (set `self.healthBarCreated?` true)
    (bind _returnvalue_2 (`GameplayStatics.SpawnSound2D` (`self.KhaimeraCue`) 1.0 1.0 0.0 null))
    (set `self.KhaimeraAudioComponent` _returnvalue_2)
    (bind _asplayer (cast `/Game/Player` (`GameplayStatics.GetPlayerCharacter` 0)))
    (`AudioComponent.FadeOut` (`/Game/Player.DungeonAudioComponent` _asplayer) 3.0 0.0 "Linear"))
  (`|ExecutionSequence`
    (:`then_0`
      (`self.HealthBarRestartTimer`))
    (:`then_1`
      (bind (_outactors _returnvalue_3) (`KismetSystemLibrary.SphereOverlapActors` (`SceneComponent.K2_GetComponentLocation` (`self.DamageArrow`)) (`self.DamageRadius`) (`|MakeArray` "ObjectTypeQuery3" :!type "EObjectTypeQuery Enum") null (`|MakeArray` self :!type "Actor Object Reference")))
      (if _returnvalue_3
        (for _array_element _outactors
          (if (`self.ActorHasTag` _array_element "Player")
            (`GameplayStatics.ApplyDamage` _array_element 20.0 (`self.GetController`) self)
            (`self.HealthBarRestartTimer`)))))))

(event `self.ReceiveAnyDamage`
  (params (Damage :type "Float (single-precision)") (DamageType :type "DamageType Object Reference") (InstigatedBy :type "Controller Object Reference") (DamageCauser :type "Actor Object Reference"))
  ;[0.7846 0.5094 1] Getting Hit/ Health Increments + Animation/Reaction to Gettting Hit
  (bind _output_get (set `self.Health` (- (`self.Health`) Damage)))
  (`AddComponent|NODE_AddParticleSystemComponent-1`)
  (if (<= (`self.Health`) (`self.zero`))
    (`Widget.RemoveFromParent` (`self.KhimeraHealthBar`))
    (`GameplayStatics.PlaySoundAtLocation` "/Game/SoundForKeyStone/Lion_Growling-SoundBible_com-657113062.Lion_Growling-SoundBible_com-657113062" (`self.K2_GetActorLocation`) (struct) 1.0 1.0 0.0 null null null)
    (`self.Kill Enemy`)
    (`AudioComponent.FadeOut` (`self.KhaimeraAudioComponent`) 3.0 0.0 "Linear")
    (bind _asplayer (cast `/Game/Player` (`GameplayStatics.GetPlayerCharacter` 0)))
    (set `/Game/Player.TargetLocked` false _asplayer)
    (`GameplayStatics.PlaySound2D` (`/Game/Player.DungeonCue` _asplayer) 1.0 1.0 0.0 null null)))

(event `Kill Enemy`
  ;[1 1 1] Ragdolls the enemy
  (`self.Ragdoll_Death`)
  (`KismetSystemLibrary.Delay` 2.0)
  (`self.K2_DestroyActor`))

(event `/Game/Evan/KeystoneImport/LockOn/LockOnBPI.LockOnReticle`
  (params (`Locked On?` :type Boolean))
  (bind _lockon (`self.LockOn`))
  ;[1 1 1] LockOn with Reticle
  (if `Locked On?`
    (`SceneComponent.SetHiddenInGame` _lockon false false)
    (else
      (`SceneComponent.SetHiddenInGame` _lockon true false))))

(fn `Ragdoll_Death`
  (`PrimitiveComponent.SetSimulatePhysics` (`self.Mesh`) true)
  (`CharacterMovementComponent.DisableMovement` (`self.CharacterMovement`)))

(fn `UserConstructionScript`)