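; Interactable chest Blueprint that animates its lid and shows a chest inventory alongside the player's inventory.
; BeginPlay creates the chest widget and fills it from ChestItems, briefly adding it to the viewport.
; Overlapping the collision enables input, so E flip-flops between opening and closing, which rotates the lid, toggles both widgets and switches cursor, input mode and movement.
; AssignChestColours applies per-instance materials but is not called within this Blueprint.
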(event `OpenChest`
  (bind _returnvalue (`GameplayStatics.GetPlayerController` 0))
  (bind _chestinventorywg (`self.ChestInventoryWG`))
  ;[1 1 1] Open + Close Chest
  (`KismetSystemLibrary.MoveComponentTo` (`self.ChestRotator`) (`SceneComponent.RelativeLocation` (`self.ChestRotator`)) (struct :`Roll` -110.0) true true 1.0)
  (`UserWidget.AddToViewport` _chestinventorywg 0)
  (set `PlayerController.bShowMouseCursor` true _returnvalue)
  (`WidgetBlueprintLibrary.SetInputMode_GameAndUIEx` _returnvalue _chestinventorywg)
  (`Controller.SetIgnoreMoveInput` _returnvalue true)
  (`UserWidget.AddToViewport` (`/Game/Player.Inventory` (cast `/Game/Player` (`GameplayStatics.GetPlayerCharacter` 0) :!pure true)) 0))

(event `CloseChest`
  (bind _returnvalue (`GameplayStatics.GetPlayerController` 0))
  ;[1 1 1] Open + Close Chest
  (`Widget.RemoveFromParent` (`self.ChestInventoryWG`))
  (set `PlayerController.bShowMouseCursor` false _returnvalue)
  (`WidgetBlueprintLibrary.SetInputMode_GameOnly` _returnvalue)
  (`Controller.SetIgnoreMoveInput` _returnvalue false)
  (`Widget.RemoveFromParent` (`/Game/Player.Inventory` (cast `/Game/Player` (`GameplayStatics.GetPlayerCharacter` 0) :!pure true)))
  (`KismetSystemLibrary.MoveComponentTo` (`self.ChestRotator`) (`SceneComponent.RelativeLocation` (`self.ChestRotator`)) (struct) true true 1.0))

(event `self.ReceiveBeginPlay`
  ;[1 1 1] BeginPlay
  (bind _returnvalue (`|CreateWidget` "/Game/InventorySystem/UI/ChestInventoryWG.ChestInventoryWG_C"))
  (set `self.ChestInventoryWG` _returnvalue)
  (`UserWidget.AddToViewport` _returnvalue 0)
  (`/Game/InventorySystem/UI/ChestInventoryWG.FillChest` (`self.ChestInventoryWG`) (`self.Chest_Items`))
  (`Widget.RemoveFromParent` _returnvalue))

(event `self.ChestCollision.OnComponentBeginOverlap`
  (params (OverlappedComponent :type "PrimitiveComponent Object Reference") (OtherActor :type "Actor Object Reference") (OtherComp :type "PrimitiveComponent Object Reference") (OtherBodyIndex :type Integer) (bFromSweep :type Boolean) (SweepResult :type "HitResult Structure (by ref)"))
  ;[1 1 1] Overlap --> Fire Open/Close Chest Event
  (`self.EnableInput` (`GameplayStatics.GetPlayerController` 0)))

(event `self.ChestCollision.OnComponentEndOverlap`
  (params (OverlappedComponent :type "PrimitiveComponent Object Reference") (OtherActor :type "Actor Object Reference") (OtherComp :type "PrimitiveComponent Object Reference") (OtherBodyIndex :type Integer))
  ;[1 1 1] Overlap --> Fire Open/Close Chest Event
  (`self.DisableInput` (`GameplayStatics.GetPlayerController` 0)))

(event `AssignChestColours`
  ;[1 1 1] Colours - Set These In The Level (Click On Your Blueprint and look at the details settings)
  (`|ExecutionSequence`
    (:`then_0`
      (`PrimitiveComponent.SetMaterial` (`self.ChestTop`) 0 (`self.TopMetalMaterial`)))
    (:`then_1`
      (`PrimitiveComponent.SetMaterial` (`self.ChestTop`) 1 (`self.TopWoodMaterial`)))
    (:`then_2`
      (`PrimitiveComponent.SetMaterial` (`self.ChestTop`) 2 (`self.TopKeyMaterial`)))
    (:`then_3`
      (`PrimitiveComponent.SetMaterial` (`self.ChestBottom`) 0 (`self.BottomMetalMaterial`)))
    (:`then_4`
      (`PrimitiveComponent.SetMaterial` (`self.ChestBottom`) 1 (`self.BottomWoodMaterial`)))))

(event `Key|E`
  (params (Key :type "Key Structure"))
  ;[1 1 1] Overlap --> Fire Open/Close Chest Event
  (:`Pressed`
    (`/Engine/EditorBlueprintResources/StandardMacros.FlipFlop`
      (:`A`
        (`self.OpenChest`))
      (:`B`
        (`self.CloseChest`)))))

(fn `UserConstructionScript`)