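; Landmine actor that arms a delayed fire explosion when its box trigger is overlapped by the Player.
; A DoOnce ahead of the Player cast lets only the first overlap through, then a sound plays and the cube's dynamic material turns red.
; After a delay it spawns temporary fire, destroys cube and box, then damages the triggering player once per actor still reported overlapping.
; DetonateTimer decrements StartDuration but is not called here.
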(event `self.Box.OnComponentBeginOverlap`
  (params (OverlappedComponent :type "PrimitiveComponent Object Reference") (OtherActor :type "Actor Object Reference") (OtherComp :type "PrimitiveComponent Object Reference") (OtherBodyIndex :type Integer) (bFromSweep :type Boolean) (SweepResult :type "HitResult Structure (by ref)"))
  (bind _returnvalue (`self.K2_GetActorLocation`))
  (`/Engine/EditorBlueprintResources/StandardMacros.DoOnce` false
    (:`Completed`
      (bind _asplayer (cast `/Game/Player` OtherActor))
      (`GameplayStatics.PlaySoundAtLocation` "/Game/SoundForKeyStone/Mine/Time_Bomb-SoundBible_com-1222708645.Time_Bomb-SoundBible_com-1222708645" _returnvalue (struct) 1.0 1.0 3.3 null null null)
      (`MaterialInstanceDynamic.SetVectorParameterValue` (`self.Color`) "Color" (struct :`R` 1.0 :`A` 1.0))
      (`KismetSystemLibrary.Delay` 1.75)
      (bind _returnvalue_2 (`GameplayStatics.SpawnEmitterAtLocation` "/Game/MedievalDungeon/Particles/P_Pit_Fire.P_Pit_Fire" _returnvalue (struct) (10.0 10.0 10.0) false))
      (`ActorComponent.K2_DestroyComponent` (`self.Cube`))
      (`ActorComponent.K2_DestroyComponent` (`self.Box`))
      (for _ (`self.GetOverlappingActors` null)
        (`GameplayStatics.ApplyDamage` _asplayer 10.0))
      (`KismetSystemLibrary.Delay` 1.5)
      (`ActorComponent.K2_DestroyComponent` _returnvalue_2))))

(fn `detonateTimer`
  (set `self.StartDuration` (- (`self.StartDuration`) 1)))

(fn `UserConstructionScript`
  (bind _returnvalue (`PrimitiveComponent.CreateDynamicMaterialInstance` (`self.Cube`) 0 null "None"))
  (set `self.Color` _returnvalue))