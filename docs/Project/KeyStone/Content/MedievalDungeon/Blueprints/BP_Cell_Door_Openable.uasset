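; Openable dungeon cell door that the player toggles open and closed with the Interact input.
; BeginPlay enables input, and a Box overlap with Player opens or closes a Gate that filters the key press.
; A FlipFlop alternates between two timelines that lerp the door mesh's yaw between closed and open angles.
; The Open flag guards each branch and updates after a three-second delay triggered from timeline updates.
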(event `self.ReceiveBeginPlay`
  ;[1 1 1] Enable Input
  (`self.EnableInput` (`GameplayStatics.GetPlayerController` 0)))

(event `InputAction|Interact` :consume false
  (params (Key :type "Key Structure"))
  ;[1 1 1] Interact
  (:`Pressed`
    (`/Engine/EditorBlueprintResources/StandardMacros.Gate` true :!label _label
      (:`Exit`
        (`/Engine/EditorBlueprintResources/StandardMacros.FlipFlop`
          (:`A`
            ;[1 1 1] Doors Open
            (if (not (`self.Open?`))
              (bind (_direction _left_door_open) (`Timeline|Timeline_0` :!via `PlayFromStart`)
                (:`Update`
                  (`SceneComponent.K2_SetRelativeRotation` (`self.SM_Cell_Door`) (`KismetMathLibrary.MakeRotator` 0.0 0.0 (`KismetMathLibrary.Lerp` (`self.Doop closed`) (`self.Door Open`) _left_door_open)) false false)
                  (`KismetSystemLibrary.Delay` 3.0)
                  (set `self.Open?` true)))))
          (:`B`
            ;[1 1 1] Door Close
            (if (`self.Open?`)
              (bind (_direction_2 _left_door_open_2) (`Timeline|Timeline_1` :!via `ReverseFromEnd`)
                (:`Update`
                  (`SceneComponent.K2_SetRelativeRotation` (`self.SM_Cell_Door`) (`KismetMathLibrary.MakeRotator` 0.0 0.0 (`KismetMathLibrary.Lerp` (`self.Doop closed`) (`self.Door Open`) _left_door_open_2)) false false)
                  (`KismetSystemLibrary.Delay` 3.0)
                  (set `self.Open?` false))))))))))

(event `self.Box.OnComponentBeginOverlap`
  (params (OverlappedComponent :type "PrimitiveComponent Object Reference") (OtherActor :type "Actor Object Reference") (OtherComp :type "PrimitiveComponent Object Reference") (OtherBodyIndex :type Integer) (bFromSweep :type Boolean) (SweepResult :type "HitResult Structure (by ref)"))
  ;[1 1 1] Interact
  (cast `/Game/Player` OtherActor)
  (goto _label :!via `Open`))

(event `self.Box.OnComponentEndOverlap`
  (params (OverlappedComponent :type "PrimitiveComponent Object Reference") (OtherActor :type "Actor Object Reference") (OtherComp :type "PrimitiveComponent Object Reference") (OtherBodyIndex :type Integer))
  ;[1 1 1] Interact
  (cast `/Game/Player` OtherActor)
  (goto _label :!via `Close`))

(fn `UserConstructionScript`)