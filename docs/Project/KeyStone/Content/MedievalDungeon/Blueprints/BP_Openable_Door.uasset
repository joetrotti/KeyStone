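; Interactive double door for the medieval dungeon that the player opens and closes with the Interact input.
; A box overlap with the Player opens or closes a gate on that input, and a FlipFlop alternates between opening and closing.
; Separate timelines for each leaf and direction lerp door yaw between closed and open values.
; An Open flag, updated after a short delay, guards each branch.
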(event `self.ReceiveBeginPlay`
  ;[1 1 1] Enable Input
  (`self.EnableInput` (`GameplayStatics.GetPlayerController` 0)))

(event `InputAction|Interact` :consume false
  (params (Key :type "Key Structure"))
  ;[1 1 1] Interact
  (:`Pressed`
    (`/Engine/EditorBlueprintResources/StandardMacros.Gate` true :!label _label
      (:`Exit`
        (`/Engine/EditorBlueprintResources/StandardMacros.FlipFlop`
          (:`A`
            ;[1 1 1] Doors Open
            (if (not (`self.Open?`))
              (`|ExecutionSequence`
                (:`then_0`
                  (bind (_direction _left_door_open) (`Timeline|Left Door Open` :!via `PlayFromStart`)
                    (:`Update`
                      (`SceneComponent.K2_SetRelativeRotation` (`self.SM_DoorWay_Large_Door_Left`) (`KismetMathLibrary.MakeRotator` 0.0 0.0 (`KismetMathLibrary.Lerp` (`self.Left Door Close Float`) (`self.Left Door Open Float`) _left_door_open)) false false))))
                (:`then_1`
                  (bind (_direction_2 _right_door_open) (`Timeline|Right Door Open` :!via `PlayFromStart`)
                    (:`Update`
                      (`SceneComponent.K2_SetRelativeRotation` (`self.SM_DoorWay_Large_Door_Right`) (`KismetMathLibrary.MakeRotator` 0.0 0.0 (`KismetMathLibrary.Lerp` (`self.Right Door Close Float`) (`self.Right Door Open Float`) _right_door_open)) false false)))))
              (`KismetSystemLibrary.Delay` 1.0)
              (set `self.Open?` true)))
          (:`B`
            ;[1 1 1] Doors Close
            (if (`self.Open?`)
              (`|ExecutionSequence`
                (:`then_0`
                  (bind (_direction_3 _left_door_open_2) (`Timeline|Timeline_0` :!via `ReverseFromEnd`)
                    (:`Update`
                      (`SceneComponent.K2_SetRelativeRotation` (`self.SM_DoorWay_Large_Door_Left`) (`KismetMathLibrary.MakeRotator` 0.0 0.0 (`KismetMathLibrary.Lerp` (`self.Left Door Close Float`) (`self.Left Door Open Float`) _left_door_open_2)) false false))))
                (:`then_1`
                  (bind (_direction_4 _right_door_open_2) (`Timeline|Timeline_1` :!via `ReverseFromEnd`)
                    (:`Update`
                      (`SceneComponent.K2_SetRelativeRotation` (`self.SM_DoorWay_Large_Door_Right`) (`KismetMathLibrary.MakeRotator` 0.0 0.0 (`KismetMathLibrary.Lerp` (`self.Right Door Close Float`) (`self.Right Door Open Float`) _right_door_open_2)) false false)))))
              (`KismetSystemLibrary.Delay` 1.0)
              (set `self.Open?` false))))))))

(event `self.Box.OnComponentBeginOverlap`
  (params (OverlappedComponent :type "PrimitiveComponent Object Reference") (OtherActor :type "Actor Object Reference") (OtherComp :type "PrimitiveComponent Object Reference") (OtherBodyIndex :type Integer) (bFromSweep :type Boolean) (SweepResult :type "HitResult Structure (by ref)"))
  ;[1 1 1] Interact
  (cast `/Game/Player` OtherActor)
  (goto _label :!via `Open`))

(event `self.Box.OnComponentEndOverlap`
  (params (OverlappedComponent :type "PrimitiveComponent Object Reference") (OtherActor :type "Actor Object Reference") (OtherComp :type "PrimitiveComponent Object Reference") (OtherBodyIndex :type Integer))
  ;[1 1 1] Interact
  (cast `/Game/Player` OtherActor)
  (goto _label :!via `Close`))

(fn `UserConstructionScript`)