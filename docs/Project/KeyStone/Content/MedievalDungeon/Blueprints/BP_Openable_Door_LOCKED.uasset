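; Double dungeon door that the player opens with the Interact input while standing in its trigger box.
; Box overlap by the ThirdPersonCharacter enables input on the actor, and Interact plays the Right and Left timelines that drive each door mesh's relative yaw.
; Leaving the box disables input and reverses both timelines to close the doors.
; Despite the LOCKED name, the graph contains no lock or key check.
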(event `self.Box.OnComponentBeginOverlap`
  (params (OverlappedComponent :type "PrimitiveComponent Object Reference") (OtherActor :type "Actor Object Reference") (OtherComp :type "PrimitiveComponent Object Reference") (OtherBodyIndex :type Integer) (bFromSweep :type Boolean) (SweepResult :type "HitResult Structure (by ref)"))
  (cast `/Game/ThirdPersonBP/Blueprints/ThirdPersonCharacter` OtherActor)
  (`self.EnableInput` (`GameplayStatics.GetPlayerController` 0)))

(event `InputAction|Interact`
  (params (Key :type "Key Structure"))
  (:`Pressed`
    (`|ExecutionSequence`
      (:`then_0`
        (bind (_direction _newtrack_0) (`Timeline|right` :!label _label)
          (:`Update`
            (`SceneComponent.K2_SetRelativeRotation` (`self.SM_DoorWay_Large_Door_Right`) (`KismetMathLibrary.MakeRotator` 0.0 0.0 _newtrack_0) false false))))
      (:`then_1`
        (bind (_direction_2 _newtrack_0_2) (`Timeline|left` :!label _label_2)
          (:`Update`
            (`SceneComponent.K2_SetRelativeRotation` (`self.SM_DoorWay_Large_Door_Left`) (`KismetMathLibrary.MakeRotator` 0.0 0.0 _newtrack_0_2) false false)))))))

(event `self.Box.OnComponentEndOverlap`
  (params (OverlappedComponent :type "PrimitiveComponent Object Reference") (OtherActor :type "Actor Object Reference") (OtherComp :type "PrimitiveComponent Object Reference") (OtherBodyIndex :type Integer))
  (cast `/Game/ThirdPersonBP/Blueprints/ThirdPersonCharacter` OtherActor)
  (`self.DisableInput` (`GameplayStatics.GetPlayerController` 0))
  (`|ExecutionSequence`
    (:`then_0`
      (goto _label :!via `Reverse`))
    (:`then_1`
      (goto _label_2 :!via `Reverse`))))

(fn `UserConstructionScript`)