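; Interactive ornate chest for the medieval dungeon that opens when the player presses Interact nearby and closes when they leave.
; Box overlap enables player input and opens a gate, which lets Interact play a timeline.
; The timeline offsets the lid mesh's world roll from the rotation cached at BeginPlay.
; End overlap disables input and reverses the timeline, though the gate is never closed again.
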(event `self.ReceiveBeginPlay`
  (set `self.InitLodRot` (`SceneComponent.K2_GetComponentRotation` (`self.SM_OrnateChest_01d`))))

(event `InputAction|Interact`
  (params (Key :type "Key Structure"))
  (bind (_initlodrot_roll _initlodrot_pitch _initlodrot_yaw) (`KismetMathLibrary.BreakRotator` (`self.InitLodRot`)))
  (:`Pressed`
    (`/Engine/EditorBlueprintResources/StandardMacros.Gate` true :!label _label
      (:`Exit`
        (bind (_direction _newtrack_0) (`Timeline|Timeline_0` :!label _label_2)
          (:`Update`
            (`SceneComponent.K2_SetWorldRotation` (`self.SM_OrnateChest_01d`) (`KismetMathLibrary.MakeRotator` (+ _initlodrot_roll _newtrack_0) _initlodrot_pitch _initlodrot_yaw) false false)))))))

(event `self.Box.OnComponentBeginOverlap`
  (params (OverlappedComponent :type "PrimitiveComponent Object Reference") (OtherActor :type "Actor Object Reference") (OtherComp :type "PrimitiveComponent Object Reference") (OtherBodyIndex :type Integer) (bFromSweep :type Boolean) (SweepResult :type "HitResult Structure (by ref)"))
  (`self.EnableInput` (`GameplayStatics.GetPlayerController` 0))
  (goto _label :!via `Open`))

(event `self.Box.OnComponentEndOverlap`
  (params (OverlappedComponent :type "PrimitiveComponent Object Reference") (OtherActor :type "Actor Object Reference") (OtherComp :type "PrimitiveComponent Object Reference") (OtherBodyIndex :type Integer))
  (`self.DisableInput` (`GameplayStatics.GetPlayerController` 0))
  (goto _label_2 :!via `Reverse`))

(fn `UserConstructionScript`)