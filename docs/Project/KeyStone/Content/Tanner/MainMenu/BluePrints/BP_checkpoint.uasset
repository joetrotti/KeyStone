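; Checkpoint actor that saves the game when anything overlaps its sphere collision.
; On overlap it prints a message, creates a fresh MySaveGame and stores the checkpoint's own transform as the player location.
; It then writes that object asynchronously to the slot and user index held in the save object.
; The construction script assigns a dynamic material instance to the cylinder mesh, with no parameters changed here.
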(event `self.Sphere_coll.OnComponentBeginOverlap`
  (params (OverlappedComponent :type "PrimitiveComponent Object Reference") (OtherActor :type "Actor Object Reference") (OtherComp :type "PrimitiveComponent Object Reference") (OtherBodyIndex :type Integer) (bFromSweep :type Boolean) (SweepResult :type "HitResult Structure (by ref)"))
  ;[1 1 1] Save Game when hit checkpoint
  (`KismetSystemLibrary.PrintString` "Checkpoint")
  (bind _returnvalue (`GameplayStatics.CreateSaveGameObject` "/Game/Tanner/SaveGame/MySaveGame.MySaveGame_C"))
  (bind _output_get (set `self.SaveGameInstance` _returnvalue))
  (set `/Game/Tanner/SaveGame/MySaveGame.PlrLocation` (`self.GetTransform`) _output_get)
  (`AsyncActionHandleSaveGame.AsyncSaveGameToSlot` _output_get (`/Game/Tanner/SaveGame/MySaveGame.Save1` _output_get) (`/Game/Tanner/SaveGame/MySaveGame.Save1Index` _output_get)))

(fn `UserConstructionScript`
  (bind _returnvalue (`KismetMaterialLibrary.CreateDynamicMaterialInstance` null))
  (set `self.Dynamic_MI_Ref` _returnvalue)
  (`PrimitiveComponent.SetMaterial` (`self.SM_cylinder`) 0 (`self.Dynamic_MI_Ref`)))